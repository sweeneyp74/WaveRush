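; Game instance for Wave Rush that owns the persistent high-score save.
; On Init it loads the wr_savegame from the highScore slot, or creates one with a zeroed score and saves it.
; The updateHighScore event overwrites the stored score and saves to the slot immediately, without comparing it to the previous value.
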(event `self.ReceiveInit`
  (bind _returnvalue (`GameplayStatics.DoesSaveGameExist` "highScore"))
  (if _returnvalue
    (bind _returnvalue_2 (`GameplayStatics.LoadGameFromSlot` "highScore"))
    (bind _aswr_savegame (cast `/Game/Blueprints/Game/wr_savegame` _returnvalue_2))
    (set `self.save_game` _aswr_savegame)
    (else
      (bind _returnvalue_3 (`GameplayStatics.CreateSaveGameObject` "/Game/Blueprints/Game/wr_savegame.wr_savegame_C"))
      (bind _output_get (set `self.save_game` _returnvalue_3))
      (set `/Game/Blueprints/Game/wr_savegame.highScore` 0.0 _output_get)
      (`GameplayStatics.SaveGameToSlot` _output_get "highScore"))))

(event `updateHighScore`
  (params (newHighScore :type "Float (double-precision)"))
  (bind _save_game (`self.save_game`))
  (set `/Game/Blueprints/Game/wr_savegame.highScore` newHighScore _save_game)
  (`GameplayStatics.SaveGameToSlot` _save_game "highScore"))