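; Spawn point actor that spawns endless, growing waves of AI-controlled pawns, starting on BeginPlay.
; Each wave spawns NumberOfPawns pawns at the particle system's location, adjusting for collisions, and gives each its default controller.
; SpawnPawn re-calls itself after a RespawnTime delay, adding one pawn per wave.
; Logic to shorten the delay down to a one-second floor exists but is unwired.
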(event `self.ReceiveBeginPlay`
  (`self.Spawn Pawn`))

(event `Spawn Pawn`
  (`self.spawnThePawns`)
  (`KismetSystemLibrary.Delay` (`self.RespawnTime`))
  (set `self.numberOfPawns` (+ (`self.numberOfPawns`) 1))
  (`self.Spawn Pawn`))

(fn `spawnThePawns`
  (for _ (range 1 (+ (`self.numberOfPawns`) 1))
    (bind _returnvalue (`|SpawnActorFromClass` "/Game/Blueprints/pawn.pawn_C" (`KismetMathLibrary.Conv_VectorToTransform` (`SceneComponent.K2_GetComponentLocation` (`self.ParticleSystem`))) "AdjustIfPossibleButAlwaysSpawn" "OverrideRootScale" null null))
    (`Pawn.SpawnDefaultController` _returnvalue))
  (`KismetSystemLibrary.PrintString` "wave spawned"))

(fn `UserConstructionScript`)