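; First-person player character for a survival shooter, handling movement, jumping, automatic gunfire, health and game over.
; Holding Shoot loops a recoil timeline, each cycle firing a camera line trace that spawns impact particles, damages hit pawns and launches them randomly.
; Incoming damage updates the HUD and grants brief immunity.
; Death disables input, records survival time as a possible high score through the game instance, then returns to the main menu.
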(event `InputAxis|MoveForward`
  (params (AxisValue :type "Float (single-precision)"))
  (`self.AddMovementInput` (`SceneComponent.GetForwardVector` (`self.CapsuleComponent`)) AxisValue))

(event `self.ReceiveBeginPlay`
  (bind _returnvalue (`|CreateWidget` "/Game/Blueprints/PlayerStuff/playerHUD.playerHUD_C"))
  (bind _output_get (set `self.playerHUD` _returnvalue))
  (`UserWidget.AddToViewport` _output_get 0)
  (set `self.gunStartVector` (`SceneComponent.RelativeLocation` (`self.gun`)))
  (`ActorComponent.Deactivate` (`self.GunParticles`))
  (`WidgetBlueprintLibrary.SetInputMode_GameOnly` (`GameplayStatics.GetPlayerController` 0)))

(event `InputAxis|MoveRIght`
  (params (AxisValue :type "Float (single-precision)"))
  (`self.AddMovementInput` (`SceneComponent.GetRightVector` (`self.CapsuleComponent`)) AxisValue))

(event `self.ReceiveTick`
  (params (DeltaSeconds :type "Float (single-precision)")))

(event `InputAxis|LookUp`
  (params (AxisValue :type "Float (single-precision)"))
  (`self.AddControllerPitchInput` AxisValue))

(event `InputAxis|LookRight`
  (params (AxisValue :type "Float (single-precision)"))
  (`self.AddControllerYawInput` AxisValue))

(event `InputAction|Shoot`
  (params (Key :type "Key Structure"))
  (bind (_gunstartvector_x _gunstartvector_y _gunstartvector_z) (`KismetMathLibrary.BreakVector` (`self.gunStartVector`)))
  (bind _gunparticles (`self.GunParticles`))
  (:`Pressed`
    (if (not (`self.isShooting`))
      (`ActorComponent.Activate` _gunparticles false)
      (`self.ShootFunction` :!label _label)
      (set `self.isShooting` true)
      (bind (_direction _gun_offset) (`Timeline|Shoot_Recoil` :!via `PlayFromStart`)
        (:`Update`
          (`SceneComponent.K2_SetRelativeLocation` (`self.gun`) (`KismetMathLibrary.MakeVector` (+ _gun_offset _gunstartvector_x) _gunstartvector_y _gunstartvector_z) false false))
        (:`Finished`
          (if (`self.isShooting`)
            (goto _label))))))
  (:`Released`
    (set `self.isShooting` false)
    (`ActorComponent.Deactivate` _gunparticles)))

(event `InputAction|Jump`
  (params (Key :type "Key Structure"))
  (:`Pressed`
    (`self.Jump`)))

(event `self.OnJumped`
  (`GameplayStatics.PlaySoundAtLocation` "/Game/sound/jump.jump" (`self.K2_GetActorLocation`) (struct) 0.5))

(event `self.ReceiveAnyDamage`
  (params (Damage :type "Float (single-precision)") (DamageType :type "DamageType Object Reference") (InstigatedBy :type "Controller Object Reference") (DamageCauser :type "Actor Object Reference"))
  (bind _playerhud (`self.playerHUD`))
  (bind _returnvalue (`self.GetGameTimeSinceCreation` (`GameplayStatics.GetGameMode`)))
  (bind _gameovertext (`/Game/Blueprints/PlayerStuff/playerHUD.gameOverText` _playerhud))
  (if (not (`self.isImmune`))
    (set `self.isImmune` true)
    (bind _output_get (set `self.Health` (- (`self.Health`) Damage)))
    (set `/Game/Blueprints/PlayerStuff/playerHUD.hudhealth` (/ _output_get 100.0) (`self.playerHUD`))
    (if (<= (`self.Health`) 0.0)
      (`self.DisableInput` null)
      (`ActorComponent.Deactivate` (`self.GunParticles`))
      (set `self.isShooting` false)
      (`CapsuleComponent.SetCapsuleHalfHeight` (`self.CapsuleComponent`) 30.0 true)
      (`Widget.SetVisibility` (`/Game/Blueprints/PlayerStuff/playerHUD.timer` _playerhud) "Collapsed")
      (`self.save_highscore` _returnvalue)
      (`Widget.SetVisibility` _gameovertext "Visible")
      (`Widget.SetVisibility` (`/Game/Blueprints/PlayerStuff/playerHUD.crosshair` _playerhud) "Collapsed")
      (`TextBlock.SetText` _gameovertext (`KismetTextLibrary.Conv_StringToText` (`KismetStringLibrary.Concat_StrStr` "You resisted friendship for " (`KismetStringLibrary.Conv_DoubleToString` _returnvalue) " seconds!")))
      (`KismetSystemLibrary.Delay` 10.0)
      (`GameplayStatics.OpenLevel` "MainMenu")
      (else
        (`KismetSystemLibrary.Delay` 0.5)
        (set `self.isImmune` false)))))

(fn `save_highscore`
  (params (score :type "Float (double-precision)"))
  (bind _aswave_rush_game_instance (cast `/Game/Blueprints/Game/WaveRushGameInstance` (`GameplayStatics.GetGameInstance`) :!pure true))
  (if (> score (`/Game/Blueprints/Game/wr_savegame.highScore` (`/Game/Blueprints/Game/WaveRushGameInstance.save_game` _aswave_rush_game_instance)))
    (`/Game/Blueprints/Game/WaveRushGameInstance.updateHighScore` _aswave_rush_game_instance score)
    (`Widget.SetVisibility` (`/Game/Blueprints/PlayerStuff/playerHUD.newHighScoreText` (`self.playerHUD`)) "Visible")))

(fn `ShootFunction`
  (bind _returnvalue (`GameplayStatics.GetPlayerCameraManager` 0))
  (`GameplayStatics.PlaySoundAtLocation` "/Game/sound/gunnoise.gunnoise" (`self.K2_GetActorLocation`) (struct) 0.5 1.25)
  (bind (_outhit _returnvalue_2) (`KismetSystemLibrary.LineTraceSingle` (`self.K2_GetActorLocation` _returnvalue) (* (`self.GetActorForwardVector` _returnvalue) 99999.0) "TraceTypeQuery1"))
  (if _returnvalue_2
    (`GameplayStatics.SpawnEmitterAtLocation` "/Game/Particles/ImpactParticles.ImpactParticles" (`.ImpactPoint` (`GameplayStatics.BreakHitResult` _outhit)) (struct) (2.0 2.0 2.0))
    (bind _aspawn (cast `/Game/Blueprints/pawn` (`.HitActor` (`GameplayStatics.BreakHitResult` _outhit))))
    (`self.LaunchCharacter` _aspawn (`KismetMathLibrary.MakeVector` (`KismetMathLibrary.RandomFloatInRange` -400.0 400.0) (`KismetMathLibrary.RandomFloatInRange` -400.0 400.0) (`KismetMathLibrary.RandomFloatInRange` -500.0 500.0)) true true)
    (`GameplayStatics.ApplyDamage` _aspawn 1.0)))

(fn `UserConstructionScript`)