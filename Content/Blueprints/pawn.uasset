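; Enemy pawn that chases the player every tick, bobs on a looping timeline and repeatedly plays a randomly pitched sound.
; Overlapping its damage box damages the player and launches them along the pawn's forward vector and upward.
; Incoming damage lowers Health; when it truncates to 0 or 1, the pawn unpossesses, spawns a DeadPawn with a random impulse and destroys itself.
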(event `self.ReceiveBeginPlay`
  (`self.speak`)
  (`KismetSystemLibrary.Delay` (`KismetMathLibrary.RandomFloatInRange` 0.0 1.0))
  (set `self.startPosition` (`SceneComponent.RelativeLocation` (`self.StaticMesh`)))
  (bind (_direction _moveupdown) (`Timeline|FloatUpAndDown` :!label _label)
    (:`Update`
      (`SceneComponent.K2_SetRelativeLocation` (`self.StaticMesh`) (+ (`self.startPosition`) (`KismetMathLibrary.MakeVector` 0.0 0.0 _moveupdown)) false false))
    (:`Finished`
      (`KismetSystemLibrary.PrintString` "Restart" false false)
      (goto _label :!via `PlayFromStart`))))

(event `self.ReceiveTick`
  (params (DeltaSeconds :type "Float (single-precision)"))
  (`NavigationSystem.SimpleMoveToLocation` (`self.GetController`) (`self.K2_GetActorLocation` (cast `/Game/Blueprints/player` (`GameplayStatics.GetPlayerPawn` 0) :!pure true))))

(event `self.ReceiveAnyDamage`
  (params (Damage :type "Float (single-precision)") (DamageType :type "DamageType Object Reference") (InstigatedBy :type "Controller Object Reference") (DamageCauser :type "Actor Object Reference"))
  (set `self.health` (- (`self.health`) Damage))
  (`self.setDamageColor`))

(event `self.damageBox.OnComponentBeginOverlap`
  (params (OverlappedComponent :type "PrimitiveComponent Object Reference") (OtherActor :type "Actor Object Reference") (OtherComp :type "PrimitiveComponent Object Reference") (OtherBodyIndex :type Integer) (bFromSweep :type Boolean) (SweepResult :type "HitResult Structure (by ref)"))
  (bind _asplayer (cast `/Game/Blueprints/player` OtherActor))
  (`GameplayStatics.ApplyDamage` _asplayer 10.0)
  (`self.LaunchCharacter` _asplayer (+ (* (`SceneComponent.GetForwardVector` (`self.CapsuleComponent`)) 800.0) (0.0 0.0 300.0)) true true))

(event `speak`
  (`KismetSystemLibrary.Delay` (`KismetMathLibrary.RandomFloatInRange` 4.0 10.0))
  (`GameplayStatics.PlaySoundAtLocation` "/Game/sound/friend_.friend_" (`SceneComponent.K2_GetComponentLocation` (`self.CapsuleComponent`)) (struct) 1.0 (`KismetMathLibrary.RandomFloatInRange` 0.1 1.9) 0.0 "/Game/sound/PawnAttenutation.PawnAttenutation")
  (`self.speak`))

(fn `float`)

(fn `setDamageColor`
  (switch `int` (`KismetMathLibrary.FTrunc` (`self.health`))
    (:`0`
      _)
    (:`1`
      _))
  (`PrimitiveComponent.SetMaterial` (`self.StaticMesh`) 0 "/Game/Materials/pawn_mat3.pawn_mat3")
  (`Controller.UnPossess` (`self.GetController`))
  (bind _returnvalue (`|SpawnActorFromClass` "/Game/Blueprints/deadPawn.deadPawn_C" (`SceneComponent.K2_GetComponentToWorld` (`self.StaticMesh`)) "Undefined" "OverrideRootScale" null null))
  (`PrimitiveComponent.AddImpulse` (`/Game/Blueprints/deadPawn.StaticMesh` _returnvalue) (`KismetMathLibrary.MakeVector` (`KismetMathLibrary.RandomFloatInRange` -400.0 400.0) (`KismetMathLibrary.RandomFloatInRange` -400.0 400.0) (`KismetMathLibrary.RandomFloatInRange` -500.0 500.0)) "None" true)
  (`self.K2_DestroyActor`))

(fn `UserConstructionScript`)